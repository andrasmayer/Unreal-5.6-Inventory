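; Base NPC actor that carries a BP_NPC as a child actor and loads its dialog data from a data table.
; The construction script hides the static mesh, leaving child components unaffected.
; On BeginPlay, if the child is a BP_NPC, it reads the Dialog table's tooltip, option name and option ID columns as strings.
; Each value is trimmed to the text between the last comma and closing parenthesis, then appended to a matching array.
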(event EventBeginPlay
  (|CallParentFunction)
  (Utilities|Casting|CastToBP_NPC (Variables|/Script/Engine.ChildActorComponent|GetChildActor (Variables|Default|GetChildActor)))
  (CallFunction|BuildDatatable))

(event Collision|EventActorBeginOverlap
  (params (OtherActor :type Actor%20Object%20Reference))
  (|CallParentFunction OtherActor) ; This node is disabled and will not be called.\nDrag off pins to build functionality.
)

(event EventTick
  (params (DeltaSeconds :type Float%20%28single-precision%29))
  (|CallParentFunction DeltaSeconds) ; This node is disabled and will not be called.\nDrag off pins to build functionality.
)

(fn ConstructionScript
  (|CallParentFunction)
  (Rendering|SetVisibility (Variables|Default|GetStaticMesh) false false))

(fn BuildDatatable
  (Utilities|FlowControl|Sequence
    (:then_0
      (bind _returnvalue (Class|DataTableFunctionLibrary|GetDataTableColumnasString (Variables|Dialog|GetDialog) "Tooltip"))
      (for _array_element _returnvalue
        (Utilities|Array|Add (Variables|Dialog|GetTooltips) (.LeftS (Utilities|String|Split (.RightS (Utilities|String|Split _array_element "," "CaseSensitive" "FromEnd")) ")")))))
    (:then_1
      (bind _returnvalue_2 (Class|DataTableFunctionLibrary|GetDataTableColumnasString (Variables|Dialog|GetDialog) "Option Names"))
      (for _array_element_2 _returnvalue_2
        (Utilities|Array|Add (Variables|Dialog|GetOption%20Names) (.LeftS (Utilities|String|Split (.RightS (Utilities|String|Split _array_element_2 "," "CaseSensitive" "FromEnd")) ")")))))
    (:then_2
      (bind _returnvalue_3 (Class|DataTableFunctionLibrary|GetDataTableColumnasString (Variables|Dialog|GetDialog) "Option Ids"))
      (for _array_element_3 _returnvalue_3
        (Utilities|Array|Add (Variables|Dialog|GetOption%20Ids) (.LeftS (Utilities|String|Split (.RightS (Utilities|String|Split _array_element_3 "," "CaseSensitive" "FromEnd")) ")")))))))